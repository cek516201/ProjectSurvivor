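; BP_LevelUpChest is a pickup item that levels up the player character when touched.
; On HitCollision overlap, it checks that the other actor's class exactly matches the game mode's default pawn class.
; It then calls DoLevelUp on player pawn 0, cast to BP_ThirdPersonCharacter, rather than on the overlapping actor, and destroys itself.
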(event OnComponentBeginOverlap(HitCollision)
  (params (OverlappedComponent :type Primitive%20Component%20Object%20Reference) (OtherActor :type Actor%20Object%20Reference) (OtherComp :type Primitive%20Component%20Object%20Reference) (OtherBodyIndex :type Integer) (bFromSweep :type Boolean) (SweepResult :type Hit%20Result%20Structure%20%28by%20ref%29))
  (if (== (Utilities|GetClass OtherActor) (Variables|/Script/Engine.GameModeBase|GetDefaultPawnClass (Game|GetGameMode)))
    (bind _asbp_third_person_character (Utilities|Casting|CastToBP_ThirdPersonCharacter (Game|Player|GetPlayerPawn 0)))
    (Default|DoLevelUp _asbp_third_person_character)
    (Actor|DestroyActor)))

(fn ConstructionScript
  (|CallParentFunction))