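; BP_ItemSpawner spawns health potion pickups at a requested location, rate-limited by a cooldown.
; On BeginPlay it loads the HealthPotion row from DT_Item and starts the timer at that row's SpawnDelay.
; Tick counts the timer down.
; TrySpawnHealthPotion spawns only once it has expired, then DoSpawnHealthPotion resets it and passes the item data to the new BP_HealthPotion.
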(event EventTick
  (params (DeltaSeconds :type Float%20%28single-precision%29))
  (CallFunction|UpdateItems DeltaSeconds))

(event EventBeginPlay
  (CallFunction|InitItem))

(fn InitItem
  (bind _returnvalue (Utilities|GetDataTableRow "/Game/Item/DT_Item.DT_Item" "HealthPotion")
    (:then
      (Variables|Default|SetHealthPotion (Utilities|Struct|MakeST_ItemReference _returnvalue (.SpawnDelay (Utilities|Struct|BreakST_Item _returnvalue)))))))

(fn UpdateItems
  (params (Delta%20Seconds :type Float%20%28double-precision%29))
  (Utilities|FlowControl|Sequence
    (:then_0
      (if (> (.currenttime (Variables|Default|GetHealthPotion)) 0.0)
        (Variables|Default|SetHealthPotion (Utilities|Struct|MakeST_ItemReference (.item (Variables|Default|GetHealthPotion)) (- (.currenttime (Variables|Default|GetHealthPotion)) Delta%20Seconds)))))))

(fn DoSpawnHealthPotion
  (params (Spawn%20Location :type Vector))
  (Variables|Default|SetHealthPotion (Utilities|Struct|MakeST_ItemReference (.item (Variables|Default|GetHealthPotion)) (.SpawnDelay (Utilities|Struct|BreakST_Item (.item (Variables|Default|GetHealthPotion))))))
  (Game|SpawnActorfromClass "/Game/Item/BP_HealthPotion.BP_HealthPotion_C" (Math|Conversions|ToTransform(Vector) Spawn%20Location) "AlwaysSpawn" "MultiplyWithRoot" 0 (.item (Variables|Default|GetHealthPotion)) 0))

(fn TrySpawnHealthPotion
  (params (Spawn%20Location :type Vector))
  (if (<= (.currenttime (Variables|Default|GetHealthPotion)) 0.0)
    (CallFunction|DoSpawnHealthPotion Spawn%20Location)))