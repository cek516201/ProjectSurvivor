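; Health potion pickup that homes in on the player and restores HP when it is not full.
; Both collision overlaps accept only the game mode's default pawn class and check HP on BP_PlayerState.
; MagneticCollision starts a timeline that lerps the potion from its start location to the player's live position.
; HitCollision adds the ItemInfo amount as healing through the player state, then destroys the potion.
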(event OnComponentBeginOverlap(HitCollision)
  (params (OverlappedComponent :type Primitive%20Component%20Object%20Reference) (OtherActor :type Actor%20Object%20Reference) (OtherComp :type Primitive%20Component%20Object%20Reference) (OtherBodyIndex :type Integer) (bFromSweep :type Boolean) (SweepResult :type Hit%20Result%20Structure%20%28by%20ref%29))
  (if (== (Utilities|GetClass OtherActor) (Variables|/Script/Engine.GameModeBase|GetDefaultPawnClass (Game|GetGameMode)))
    (bind _asbp_player_state (Utilities|Casting|CastToBP_PlayerState (Game|GetPlayerState 0)))
    (if (not (Default|IsHpFull _asbp_player_state))
      (CallFunction|DoHealPlayer _asbp_player_state))))

(event OnComponentBeginOverlap(MagneticCollision)
  (params (OverlappedComponent :type Primitive%20Component%20Object%20Reference) (OtherActor :type Actor%20Object%20Reference) (OtherComp :type Primitive%20Component%20Object%20Reference) (OtherBodyIndex :type Integer) (bFromSweep :type Boolean) (SweepResult :type Hit%20Result%20Structure%20%28by%20ref%29))
  (if (== (Utilities|GetClass OtherActor) (Variables|/Script/Engine.GameModeBase|GetDefaultPawnClass (Game|GetGameMode)))
    (bind _asbp_player_state (Utilities|Casting|CastToBP_PlayerState (Game|GetPlayerState 0)))
    (if (not (Default|IsHpFull _asbp_player_state))
      (CallFunction|DoMovetoPlayer))))

(event Custom|DoMoveToPlayer
  (Variables|Default|SetMove%20Start%20Location (Transformation|GetActorLocation))
  (bind _move_alpha (Timeline|아이템%20이동%20타임라인 Play)
    (:Update
      (Transformation|SetActorLocation (Math|Vector|Lerp(Vector) (Variables|Default|GetMove%20Start%20Location) (Transformation|GetActorLocation (Game|GetPlayerCharacter 0)) _move_alpha) false false))))

(fn ConstructionScript
  (|CallParentFunction))

(fn DoHealPlayer
  (params (Player%20State :type BP%20Player%20State%20Object%20Reference%20%28by%20ref%29))
  (Default|AddHeal Player%20State (.amount (Variables|Default|GetItemInfo)))
  (Actor|DestroyActor))