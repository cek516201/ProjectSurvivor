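; BP_ShieldAura is a short-lived skill actor that spins around its instigator's position as a shield aura.
; Each Tick it adds world yaw scaled by delta time and Speed, then teleport-free, unswept SetActorLocation snaps it onto the instigator without attachment.
; A timer set by function name on BeginPlay calls DoDestroySkill to destroy it after five seconds; no collision or protection logic is in these graphs.
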(event EventTick
  (params (DeltaSeconds :type Float%20%28single-precision%29))
  (Utilities|FlowControl|Sequence
    (:then_0
      (Class|Actor|AddActorWorldRotation (Math|Rotator|MakeRotator 0.0 0.0 (* DeltaSeconds (Variables|Default|GetSpeed)))))
    (:then_1
      (Transformation|SetActorLocation (Transformation|GetActorLocation (Game|GetInstigator)) false false))))

(event EventBeginPlay
  (Utilities|Time|SetTimerbyFunctionName 0 "DoDestroySkill" 5.0))

(fn ConstructionScript)

(fn DoDestroySkill
  (Actor|DestroyActor))