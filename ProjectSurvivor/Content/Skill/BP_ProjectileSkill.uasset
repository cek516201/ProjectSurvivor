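; Projectile skill actor that flies forward and damages monsters it touches.
; Tick offsets it along its forward vector by Speed without sweeping, and a timer started on BeginPlay destroys it after a short lifetime.
; HitCollision overlaps with BP_Monster_Base actors apply SkillInfo damage credited to player controller 0.
; The projectile is not destroyed on hit, so it can pass through and damage several monsters.
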(event OnComponentBeginOverlap(HitCollision)
  (params (OverlappedComponent :type Primitive%20Component%20Object%20Reference) (OtherActor :type Actor%20Object%20Reference) (OtherComp :type Primitive%20Component%20Object%20Reference) (OtherBodyIndex :type Integer) (bFromSweep :type Boolean) (SweepResult :type Hit%20Result%20Structure%20%28by%20ref%29))
  (bind _asbp_monster_base (Utilities|Casting|CastToBP_Monster_Base OtherActor))
  (CallFunction|DoDamage _asbp_monster_base))

(event EventTick
  (params (DeltaSeconds :type Float%20%28single-precision%29))
  (Transformation|AddActorWorldOffset (* (* DeltaSeconds (Variables|Default|GetSpeed)) (Transformation|GetActorForwardVector))))

(event EventBeginPlay
  (Utilities|Time|SetTimerbyFunctionName 0 "DoDestroy" 0.5))

(fn ConstructionScript)

(fn DoDestroy
  (Actor|DestroyActor))

(fn DoDamage
  (params (TargetMonster :type BP%20Monster%20Base%20Object%20Reference))
  (Game|Damage|ApplyDamage TargetMonster (.damage (Variables|Default|GetSkillInfo)) (Game|GetPlayerController 0) self))