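; BP_SlashSkill is a slash skill actor that damages monsters caught in its sphere.
; On BeginPlay it attaches to its instigator and applies SkillInfo damage once to overlapping BP_Monster_Base actors, crediting player controller 0.
; Tick manually advances the Niagara slash simulation by twice the frame delta to speed up the effect.
; The actor destroys itself through a callback bound to the effect finishing.
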(event EventBeginPlay
  (Transformation|AttachActorToActor (Game|GetInstigator) "None" "KeepWorld" "KeepWorld" "KeepWorld" true)
  (EventDispatchers|BindEventtoOnSystemFinished (Variables|Default|GetNS_Free_Magic_Slash) (EventDispatchers|CreateEvent :!event EventEffectFinish))
  (CallFunction|DoDamage))

(event EventTick
  (params (DeltaSeconds :type Float%20%28single-precision%29))
  (Class|NiagaraComponent|AdvanceSimulation (Variables|Default|GetNS_Free_Magic_Slash) 1 (* DeltaSeconds 2.0)))

(fn ConstructionScript)

(fn EventEffectFinish
  (params (PSystem :type Niagara%20Component%20Object%20Reference))
  (Actor|DestroyActor))

(fn DoDamage
  (for _array_element (Collision|GetOverlappingActors (Variables|Default|GetSphere) "/Game/ThirdPerson/Monsters/BP_Monster_Base.BP_Monster_Base_C" :!class /Script/Engine.PrimitiveComponent)
    (Game|Damage|ApplyDamage _array_element (.damage (Variables|Default|GetSkillInfo)) (Game|GetPlayerController 0) self)))